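; Test actor that feeds samples from a float curve into a spline at BeginPlay.
; It starts at the curve's minimum time and, if below the maximum, advances by Iter and adds a spline point with time as X and curve value as Y.
; The graph shows a single conditional step with no loop back, so only one point is added.
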(event EventBeginPlay
  (bind _curve (Variables|Default|GetCurve))
  (bind (_mintime _maxtime) (Math|Curves|GetTimeRange _curve))
  (Variables|Default|SetCurrentTime _mintime)
  (if (< (Variables|Default|GetCurrentTime) _maxtime)
    (bind _output_get (Variables|Default|SetCurrentTime (+ (Variables|Default|GetIter) (Variables|Default|GetCurrentTime))))
    (Class|SplineComponent|AddPoint (Variables|Default|GetSpline) (Utilities|Struct|MakeSplinePoint 0.0 (Math|Vector|MakeVector _output_get (Math|Curves|GetFloatValue _curve (Variables|Default|GetCurrentTime)) 0.0) "0.000000,0.000000,0.000000" "0.000000,0.000000,0.000000" "0.000000,0.000000,0.000000" "1.000000,1.000000,1.000000" "Curve") true)))

(event Collision|EventActorBeginOverlap
  (params (OtherActor :type Actor%20Object%20Reference)))

(event EventTick
  (params (DeltaSeconds :type Float%20%28single-precision%29)))

(fn ConstructionScript)